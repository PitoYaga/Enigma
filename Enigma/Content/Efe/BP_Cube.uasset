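; Cube actor that turns in 90-degree steps based on which edge trigger the player pawn enters.
; Left/Right X, Y and Z collision overlaps cache the pawn, store a signed quarter-turn in CurrentRotator and set CanRotate.
; Z triggers reuse the Y rotations, with left and right swapped.
; RotateCube, not called within this graph, applies the stored rotation to CubeParent as a relative offset and clears CanRotate without checking it.
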(event OnComponentBeginOverlap(LeftXCollision6)
  (params (OverlappedComponent :type Primitive%20Component%20Object%20Reference) (OtherActor :type Actor%20Object%20Reference) (OtherComp :type Primitive%20Component%20Object%20Reference) (OtherBodyIndex :type Integer) (bFromSweep :type Boolean) (SweepResult :type Hit%20Result%20Structure%20%28by%20ref%29))
  ;[1 1 1] Left_X
  (bind _asbp_player_pawn (Utilities|Casting|CastToBP_PlayerPawn OtherActor))
  (Variables|Default|SetAs%20BP%20Player%20Pawn _asbp_player_pawn)
  (Variables|Default|SetCurrentRotator "0, 0,-90.000000")
  (Variables|Default|SetcanRotate true))

(event OnComponentBeginOverlap(LeftXCollision5)
  (params (OverlappedComponent :type Primitive%20Component%20Object%20Reference) (OtherActor :type Actor%20Object%20Reference) (OtherComp :type Primitive%20Component%20Object%20Reference) (OtherBodyIndex :type Integer) (bFromSweep :type Boolean) (SweepResult :type Hit%20Result%20Structure%20%28by%20ref%29))
  ;[1 1 1] Left_X
  (bind _asbp_player_pawn (Utilities|Casting|CastToBP_PlayerPawn OtherActor))
  (Variables|Default|SetAs%20BP%20Player%20Pawn _asbp_player_pawn)
  (Variables|Default|SetCurrentRotator "0, 0,-90.000000")
  (Variables|Default|SetcanRotate true))

(event OnComponentBeginOverlap(LeftYCollision8)
  (params (OverlappedComponent :type Primitive%20Component%20Object%20Reference) (OtherActor :type Actor%20Object%20Reference) (OtherComp :type Primitive%20Component%20Object%20Reference) (OtherBodyIndex :type Integer) (bFromSweep :type Boolean) (SweepResult :type Hit%20Result%20Structure%20%28by%20ref%29))
  ;[1 1 1] Left_Y
  (bind _asbp_player_pawn (Utilities|Casting|CastToBP_PlayerPawn OtherActor))
  (Variables|Default|SetAs%20BP%20Player%20Pawn _asbp_player_pawn)
  (Variables|Default|SetCurrentRotator "-90.000000, 0,0.000000")
  (Variables|Default|SetcanRotate true))

(event OnComponentBeginOverlap(LeftYCollision11)
  (params (OverlappedComponent :type Primitive%20Component%20Object%20Reference) (OtherActor :type Actor%20Object%20Reference) (OtherComp :type Primitive%20Component%20Object%20Reference) (OtherBodyIndex :type Integer) (bFromSweep :type Boolean) (SweepResult :type Hit%20Result%20Structure%20%28by%20ref%29))
  ;[1 1 1] Left_Y
  (bind _asbp_player_pawn (Utilities|Casting|CastToBP_PlayerPawn OtherActor))
  (Variables|Default|SetAs%20BP%20Player%20Pawn _asbp_player_pawn)
  (Variables|Default|SetCurrentRotator "-90.000000, 0,0.000000")
  (Variables|Default|SetcanRotate true))

(event OnComponentBeginOverlap(Right_Y_Collision_2)
  (params (OverlappedComponent :type Primitive%20Component%20Object%20Reference) (OtherActor :type Actor%20Object%20Reference) (OtherComp :type Primitive%20Component%20Object%20Reference) (OtherBodyIndex :type Integer) (bFromSweep :type Boolean) (SweepResult :type Hit%20Result%20Structure%20%28by%20ref%29))
  ;[1 1 1] Right_Y
  (bind _asbp_player_pawn (Utilities|Casting|CastToBP_PlayerPawn OtherActor))
  (Variables|Default|SetAs%20BP%20Player%20Pawn _asbp_player_pawn)
  (Variables|Default|SetCurrentRotator "90.000000, 0,0.000000")
  (Variables|Default|SetcanRotate true))

(event OnComponentBeginOverlap(Right_Y_Collision_3)
  (params (OverlappedComponent :type Primitive%20Component%20Object%20Reference) (OtherActor :type Actor%20Object%20Reference) (OtherComp :type Primitive%20Component%20Object%20Reference) (OtherBodyIndex :type Integer) (bFromSweep :type Boolean) (SweepResult :type Hit%20Result%20Structure%20%28by%20ref%29))
  ;[1 1 1] Right_Y
  (bind _asbp_player_pawn (Utilities|Casting|CastToBP_PlayerPawn OtherActor))
  (Variables|Default|SetAs%20BP%20Player%20Pawn _asbp_player_pawn)
  (Variables|Default|SetCurrentRotator "90.000000, 0,0.000000")
  (Variables|Default|SetcanRotate true))

(event OnComponentBeginOverlap(Right_Y_Collision)
  (params (OverlappedComponent :type Primitive%20Component%20Object%20Reference) (OtherActor :type Actor%20Object%20Reference) (OtherComp :type Primitive%20Component%20Object%20Reference) (OtherBodyIndex :type Integer) (bFromSweep :type Boolean) (SweepResult :type Hit%20Result%20Structure%20%28by%20ref%29))
  ;[1 1 1] Right_Y
  (bind _asbp_player_pawn (Utilities|Casting|CastToBP_PlayerPawn OtherActor))
  (Variables|Default|SetAs%20BP%20Player%20Pawn _asbp_player_pawn)
  (Variables|Default|SetCurrentRotator "90.000000, 0,0.000000")
  (Variables|Default|SetcanRotate true))

(event OnComponentBeginOverlap(Right_Y_Collision_1)
  (params (OverlappedComponent :type Primitive%20Component%20Object%20Reference) (OtherActor :type Actor%20Object%20Reference) (OtherComp :type Primitive%20Component%20Object%20Reference) (OtherBodyIndex :type Integer) (bFromSweep :type Boolean) (SweepResult :type Hit%20Result%20Structure%20%28by%20ref%29))
  ;[1 1 1] Right_Y
  (bind _asbp_player_pawn (Utilities|Casting|CastToBP_PlayerPawn OtherActor))
  (Variables|Default|SetAs%20BP%20Player%20Pawn _asbp_player_pawn)
  (Variables|Default|SetCurrentRotator "90.000000, 0,0.000000")
  (Variables|Default|SetcanRotate true))

(event OnComponentBeginOverlap(Right_Z_04)
  (params (OverlappedComponent :type Primitive%20Component%20Object%20Reference) (OtherActor :type Actor%20Object%20Reference) (OtherComp :type Primitive%20Component%20Object%20Reference) (OtherBodyIndex :type Integer) (bFromSweep :type Boolean) (SweepResult :type Hit%20Result%20Structure%20%28by%20ref%29))
  ;[1 1 1] Left_Y
  (bind _asbp_player_pawn (Utilities|Casting|CastToBP_PlayerPawn OtherActor))
  (Variables|Default|SetAs%20BP%20Player%20Pawn _asbp_player_pawn)
  (Variables|Default|SetCurrentRotator "-90.000000, 0,0.000000")
  (Variables|Default|SetcanRotate true))

(event OnComponentBeginOverlap(Right_Z_01)
  (params (OverlappedComponent :type Primitive%20Component%20Object%20Reference) (OtherActor :type Actor%20Object%20Reference) (OtherComp :type Primitive%20Component%20Object%20Reference) (OtherBodyIndex :type Integer) (bFromSweep :type Boolean) (SweepResult :type Hit%20Result%20Structure%20%28by%20ref%29))
  ;[1 1 1] Left_Y
  (bind _asbp_player_pawn (Utilities|Casting|CastToBP_PlayerPawn OtherActor))
  (Variables|Default|SetAs%20BP%20Player%20Pawn _asbp_player_pawn)
  (Variables|Default|SetCurrentRotator "-90.000000, 0,0.000000")
  (Variables|Default|SetcanRotate true))

(event OnComponentBeginOverlap(Right_Z_02)
  (params (OverlappedComponent :type Primitive%20Component%20Object%20Reference) (OtherActor :type Actor%20Object%20Reference) (OtherComp :type Primitive%20Component%20Object%20Reference) (OtherBodyIndex :type Integer) (bFromSweep :type Boolean) (SweepResult :type Hit%20Result%20Structure%20%28by%20ref%29))
  ;[1 1 1] Left_Y
  (bind _asbp_player_pawn (Utilities|Casting|CastToBP_PlayerPawn OtherActor))
  (Variables|Default|SetAs%20BP%20Player%20Pawn _asbp_player_pawn)
  (Variables|Default|SetCurrentRotator "-90.000000, 0,0.000000")
  (Variables|Default|SetcanRotate true))

(event OnComponentBeginOverlap(Right_Z_03)
  (params (OverlappedComponent :type Primitive%20Component%20Object%20Reference) (OtherActor :type Actor%20Object%20Reference) (OtherComp :type Primitive%20Component%20Object%20Reference) (OtherBodyIndex :type Integer) (bFromSweep :type Boolean) (SweepResult :type Hit%20Result%20Structure%20%28by%20ref%29))
  ;[1 1 1] Left_Y
  (bind _asbp_player_pawn (Utilities|Casting|CastToBP_PlayerPawn OtherActor))
  (Variables|Default|SetAs%20BP%20Player%20Pawn _asbp_player_pawn)
  (Variables|Default|SetCurrentRotator "-90.000000, 0,0.000000")
  (Variables|Default|SetcanRotate true))

(event OnComponentBeginOverlap(LeftXCollision4)
  (params (OverlappedComponent :type Primitive%20Component%20Object%20Reference) (OtherActor :type Actor%20Object%20Reference) (OtherComp :type Primitive%20Component%20Object%20Reference) (OtherBodyIndex :type Integer) (bFromSweep :type Boolean) (SweepResult :type Hit%20Result%20Structure%20%28by%20ref%29))
  ;[1 1 1] Left_X
  (bind _asbp_player_pawn (Utilities|Casting|CastToBP_PlayerPawn OtherActor))
  (Variables|Default|SetAs%20BP%20Player%20Pawn _asbp_player_pawn)
  (Variables|Default|SetCurrentRotator "0, 0,-90.000000")
  (Variables|Default|SetcanRotate true))

(event OnComponentBeginOverlap(Left_Z_02)
  (params (OverlappedComponent :type Primitive%20Component%20Object%20Reference) (OtherActor :type Actor%20Object%20Reference) (OtherComp :type Primitive%20Component%20Object%20Reference) (OtherBodyIndex :type Integer) (bFromSweep :type Boolean) (SweepResult :type Hit%20Result%20Structure%20%28by%20ref%29))
  ;[1 1 1] Right_Y
  (bind _asbp_player_pawn (Utilities|Casting|CastToBP_PlayerPawn OtherActor))
  (Variables|Default|SetAs%20BP%20Player%20Pawn _asbp_player_pawn)
  (Variables|Default|SetCurrentRotator "90.000000, 0,0.000000")
  (Variables|Default|SetcanRotate true))

(event OnComponentBeginOverlap(Left_Z_03)
  (params (OverlappedComponent :type Primitive%20Component%20Object%20Reference) (OtherActor :type Actor%20Object%20Reference) (OtherComp :type Primitive%20Component%20Object%20Reference) (OtherBodyIndex :type Integer) (bFromSweep :type Boolean) (SweepResult :type Hit%20Result%20Structure%20%28by%20ref%29))
  ;[1 1 1] Right_Y
  (bind _asbp_player_pawn (Utilities|Casting|CastToBP_PlayerPawn OtherActor))
  (Variables|Default|SetAs%20BP%20Player%20Pawn _asbp_player_pawn)
  (Variables|Default|SetCurrentRotator "90.000000, 0,0.000000")
  (Variables|Default|SetcanRotate true))

(event OnComponentBeginOverlap(Left_Z_04)
  (params (OverlappedComponent :type Primitive%20Component%20Object%20Reference) (OtherActor :type Actor%20Object%20Reference) (OtherComp :type Primitive%20Component%20Object%20Reference) (OtherBodyIndex :type Integer) (bFromSweep :type Boolean) (SweepResult :type Hit%20Result%20Structure%20%28by%20ref%29))
  ;[1 1 1] Right_Y
  (bind _asbp_player_pawn (Utilities|Casting|CastToBP_PlayerPawn OtherActor))
  (Variables|Default|SetAs%20BP%20Player%20Pawn _asbp_player_pawn)
  (Variables|Default|SetCurrentRotator "90.000000, 0,0.000000")
  (Variables|Default|SetcanRotate true))

(event OnComponentBeginOverlap(Left_Z_01)
  (params (OverlappedComponent :type Primitive%20Component%20Object%20Reference) (OtherActor :type Actor%20Object%20Reference) (OtherComp :type Primitive%20Component%20Object%20Reference) (OtherBodyIndex :type Integer) (bFromSweep :type Boolean) (SweepResult :type Hit%20Result%20Structure%20%28by%20ref%29))
  ;[1 1 1] Right_Y
  (bind _asbp_player_pawn (Utilities|Casting|CastToBP_PlayerPawn OtherActor))
  (Variables|Default|SetAs%20BP%20Player%20Pawn _asbp_player_pawn)
  (Variables|Default|SetCurrentRotator "90.000000, 0,0.000000")
  (Variables|Default|SetcanRotate true))

(event OnComponentBeginOverlap(LeftXCollision7)
  (params (OverlappedComponent :type Primitive%20Component%20Object%20Reference) (OtherActor :type Actor%20Object%20Reference) (OtherComp :type Primitive%20Component%20Object%20Reference) (OtherBodyIndex :type Integer) (bFromSweep :type Boolean) (SweepResult :type Hit%20Result%20Structure%20%28by%20ref%29))
  ;[1 1 1] Left_X
  (bind _asbp_player_pawn (Utilities|Casting|CastToBP_PlayerPawn OtherActor))
  (Variables|Default|SetAs%20BP%20Player%20Pawn _asbp_player_pawn)
  (Variables|Default|SetCurrentRotator "0, 0,-90.000000")
  (Variables|Default|SetcanRotate true))

(event OnComponentBeginOverlap(RightXCollision2)
  (params (OverlappedComponent :type Primitive%20Component%20Object%20Reference) (OtherActor :type Actor%20Object%20Reference) (OtherComp :type Primitive%20Component%20Object%20Reference) (OtherBodyIndex :type Integer) (bFromSweep :type Boolean) (SweepResult :type Hit%20Result%20Structure%20%28by%20ref%29))
  ;[1 1 1] Right_X
  (bind _asbp_player_pawn (Utilities|Casting|CastToBP_PlayerPawn OtherActor))
  (Variables|Default|SetAs%20BP%20Player%20Pawn _asbp_player_pawn)
  (Variables|Default|SetCurrentRotator "0, 0,90.000000")
  (Variables|Default|SetcanRotate true))

(event OnComponentBeginOverlap(RightXCollision)
  (params (OverlappedComponent :type Primitive%20Component%20Object%20Reference) (OtherActor :type Actor%20Object%20Reference) (OtherComp :type Primitive%20Component%20Object%20Reference) (OtherBodyIndex :type Integer) (bFromSweep :type Boolean) (SweepResult :type Hit%20Result%20Structure%20%28by%20ref%29))
  ;[1 1 1] Right_X
  (bind _asbp_player_pawn (Utilities|Casting|CastToBP_PlayerPawn OtherActor))
  (Variables|Default|SetAs%20BP%20Player%20Pawn _asbp_player_pawn)
  (Variables|Default|SetCurrentRotator "0, 0,90.000000")
  (Variables|Default|SetcanRotate true))

(event OnComponentBeginOverlap(RightXCollision1)
  (params (OverlappedComponent :type Primitive%20Component%20Object%20Reference) (OtherActor :type Actor%20Object%20Reference) (OtherComp :type Primitive%20Component%20Object%20Reference) (OtherBodyIndex :type Integer) (bFromSweep :type Boolean) (SweepResult :type Hit%20Result%20Structure%20%28by%20ref%29))
  ;[1 1 1] Right_X
  (bind _asbp_player_pawn (Utilities|Casting|CastToBP_PlayerPawn OtherActor))
  (Variables|Default|SetAs%20BP%20Player%20Pawn _asbp_player_pawn)
  (Variables|Default|SetCurrentRotator "0, 0,90.000000")
  (Variables|Default|SetcanRotate true))

(event OnComponentBeginOverlap(RightXCollision3)
  (params (OverlappedComponent :type Primitive%20Component%20Object%20Reference) (OtherActor :type Actor%20Object%20Reference) (OtherComp :type Primitive%20Component%20Object%20Reference) (OtherBodyIndex :type Integer) (bFromSweep :type Boolean) (SweepResult :type Hit%20Result%20Structure%20%28by%20ref%29))
  ;[1 1 1] Right_X
  (bind _asbp_player_pawn (Utilities|Casting|CastToBP_PlayerPawn OtherActor))
  (Variables|Default|SetAs%20BP%20Player%20Pawn _asbp_player_pawn)
  (Variables|Default|SetCurrentRotator "0, 0,90.000000")
  (Variables|Default|SetcanRotate true))

(event OnComponentBeginOverlap(LeftYCollision10)
  (params (OverlappedComponent :type Primitive%20Component%20Object%20Reference) (OtherActor :type Actor%20Object%20Reference) (OtherComp :type Primitive%20Component%20Object%20Reference) (OtherBodyIndex :type Integer) (bFromSweep :type Boolean) (SweepResult :type Hit%20Result%20Structure%20%28by%20ref%29))
  ;[1 1 1] Left_Y
  (bind _asbp_player_pawn (Utilities|Casting|CastToBP_PlayerPawn OtherActor))
  (Variables|Default|SetAs%20BP%20Player%20Pawn _asbp_player_pawn)
  (Variables|Default|SetCurrentRotator "-90.000000, 0,0.000000")
  (Variables|Default|SetcanRotate true))

(event OnComponentBeginOverlap(LeftYCollision9)
  (params (OverlappedComponent :type Primitive%20Component%20Object%20Reference) (OtherActor :type Actor%20Object%20Reference) (OtherComp :type Primitive%20Component%20Object%20Reference) (OtherBodyIndex :type Integer) (bFromSweep :type Boolean) (SweepResult :type Hit%20Result%20Structure%20%28by%20ref%29))
  ;[1 1 1] Left_Y
  (bind _asbp_player_pawn (Utilities|Casting|CastToBP_PlayerPawn OtherActor))
  (Variables|Default|SetAs%20BP%20Player%20Pawn _asbp_player_pawn)
  (Variables|Default|SetCurrentRotator "-90.000000, 0,0.000000")
  (Variables|Default|SetcanRotate true))

(event Custom|RotateCube
  (Transformation|AddRelativeRotation (Variables|Default|GetCubeParent) (Variables|Default|GetCurrentRotator) false false)
  (Variables|Default|SetcanRotate false))

(event EventBeginPlay
  (bind _asbp_player_pawn (Utilities|Casting|CastToBP_PlayerPawn (Game|Player|GetPlayerPawn 0)))
  (Variables|Default|SetAs%20BP%20Player%20Pawn _asbp_player_pawn))

(fn ConstructionScript)