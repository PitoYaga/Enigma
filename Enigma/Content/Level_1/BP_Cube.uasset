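; BP_Cube is a Level 1 cube that rotates in steps as the player pawn interacts with its trigger volumes.
; Trigger overlaps by BP_PlayerPawn_1 store a preset rotation offset in CurrentRotator and set CanRotate.
; The RotateCube event adds that offset to the root's world rotation, eases to it over one second with MoveComponentTo, then clears CanRotate.
; Actors entering the Box volume attach to the cube, keeping their world transform.
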(event OnComponentBeginOverlap(Y-90/4)
  (params (OverlappedComponent :type Primitive%20Component%20Object%20Reference) (OtherActor :type Actor%20Object%20Reference) (OtherComp :type Primitive%20Component%20Object%20Reference) (OtherBodyIndex :type Integer) (bFromSweep :type Boolean) (SweepResult :type Hit%20Result%20Structure%20%28by%20ref%29))
  ;[0.4219 0 0.01549] Y-90
  (bind _asbp_player_pawn_1 (Utilities|Casting|CastToBP_PlayerPawn_1 OtherActor))
  (Variables|Default|SetAs%20BP%20Player%20Pawn _asbp_player_pawn_1)
  (Variables|Default|SetCurrentRotator "90.000000,0.000000,0.000000")
  (Variables|Default|SetcanRotate true))

(event OnComponentBeginOverlap(Y-90/3)
  (params (OverlappedComponent :type Primitive%20Component%20Object%20Reference) (OtherActor :type Actor%20Object%20Reference) (OtherComp :type Primitive%20Component%20Object%20Reference) (OtherBodyIndex :type Integer) (bFromSweep :type Boolean) (SweepResult :type Hit%20Result%20Structure%20%28by%20ref%29))
  ;[0.4219 0 0.01549] Y-90
  (bind _asbp_player_pawn_1 (Utilities|Casting|CastToBP_PlayerPawn_1 OtherActor))
  (Variables|Default|SetAs%20BP%20Player%20Pawn _asbp_player_pawn_1)
  (Variables|Default|SetCurrentRotator "-90.000000, 0,0.000000")
  (Variables|Default|SetcanRotate true))

(event OnComponentBeginOverlap(Y-90/1)
  (params (OverlappedComponent :type Primitive%20Component%20Object%20Reference) (OtherActor :type Actor%20Object%20Reference) (OtherComp :type Primitive%20Component%20Object%20Reference) (OtherBodyIndex :type Integer) (bFromSweep :type Boolean) (SweepResult :type Hit%20Result%20Structure%20%28by%20ref%29))
  (bind _asbp_player_pawn_1 (Utilities|Casting|CastToBP_PlayerPawn_1 OtherActor))
  (Variables|Default|SetAs%20BP%20Player%20Pawn _asbp_player_pawn_1)
  (Variables|Default|SetCurrentRotator "-90.000000,180.000000,180.000000")
  (Variables|Default|SetcanRotate true))

(event OnComponentBeginOverlap(Y-90/2)
  (params (OverlappedComponent :type Primitive%20Component%20Object%20Reference) (OtherActor :type Actor%20Object%20Reference) (OtherComp :type Primitive%20Component%20Object%20Reference) (OtherBodyIndex :type Integer) (bFromSweep :type Boolean) (SweepResult :type Hit%20Result%20Structure%20%28by%20ref%29))
  (bind _asbp_player_pawn_1 (Utilities|Casting|CastToBP_PlayerPawn_1 OtherActor))
  (Variables|Default|SetAs%20BP%20Player%20Pawn _asbp_player_pawn_1)
  (Variables|Default|SetCurrentRotator "-90.000000,180.000000,180.000000")
  (Variables|Default|SetcanRotate true))

(event OnComponentBeginOverlap(Y+90/3)
  (params (OverlappedComponent :type Primitive%20Component%20Object%20Reference) (OtherActor :type Actor%20Object%20Reference) (OtherComp :type Primitive%20Component%20Object%20Reference) (OtherBodyIndex :type Integer) (bFromSweep :type Boolean) (SweepResult :type Hit%20Result%20Structure%20%28by%20ref%29))
  ;[0 0.4219 0.05633] Y+90
  (bind _asbp_player_pawn_1 (Utilities|Casting|CastToBP_PlayerPawn_1 OtherActor))
  (Variables|Default|SetAs%20BP%20Player%20Pawn _asbp_player_pawn_1)
  (Variables|Default|SetCurrentRotator "90.000000,0.000000,0.000000")
  (Variables|Default|SetcanRotate true))

(event OnComponentBeginOverlap(Y+90/4)
  (params (OverlappedComponent :type Primitive%20Component%20Object%20Reference) (OtherActor :type Actor%20Object%20Reference) (OtherComp :type Primitive%20Component%20Object%20Reference) (OtherBodyIndex :type Integer) (bFromSweep :type Boolean) (SweepResult :type Hit%20Result%20Structure%20%28by%20ref%29))
  ;[0 0.4219 0.05633] Y+90
  (bind _asbp_player_pawn_1 (Utilities|Casting|CastToBP_PlayerPawn_1 OtherActor))
  (Variables|Default|SetAs%20BP%20Player%20Pawn _asbp_player_pawn_1)
  (Variables|Default|SetCurrentRotator "-90.000000,0.000000,-360.000000")
  (Variables|Default|SetcanRotate true))

(event OnComponentBeginOverlap(Y+90/1)
  (params (OverlappedComponent :type Primitive%20Component%20Object%20Reference) (OtherActor :type Actor%20Object%20Reference) (OtherComp :type Primitive%20Component%20Object%20Reference) (OtherBodyIndex :type Integer) (bFromSweep :type Boolean) (SweepResult :type Hit%20Result%20Structure%20%28by%20ref%29))
  ;[0 0.4219 0.05633] Y+90
  (bind _asbp_player_pawn_1 (Utilities|Casting|CastToBP_PlayerPawn_1 OtherActor))
  (Variables|Default|SetAs%20BP%20Player%20Pawn _asbp_player_pawn_1)
  (Variables|Default|SetCurrentRotator "90.000000,180.000000,180.000000")
  (Variables|Default|SetcanRotate true))

(event OnComponentBeginOverlap(Y+90/2)
  (params (OverlappedComponent :type Primitive%20Component%20Object%20Reference) (OtherActor :type Actor%20Object%20Reference) (OtherComp :type Primitive%20Component%20Object%20Reference) (OtherBodyIndex :type Integer) (bFromSweep :type Boolean) (SweepResult :type Hit%20Result%20Structure%20%28by%20ref%29))
  (bind _asbp_player_pawn_1 (Utilities|Casting|CastToBP_PlayerPawn_1 OtherActor))
  (Variables|Default|SetAs%20BP%20Player%20Pawn _asbp_player_pawn_1)
  (Variables|Default|SetCurrentRotator "90.000000,-180.000000,-180.000000")
  ;[0 0.4219 0.05633] Y+90
  (Variables|Default|SetcanRotate true))

(event OnComponentBeginOverlap(X+90/1)
  (params (OverlappedComponent :type Primitive%20Component%20Object%20Reference) (OtherActor :type Actor%20Object%20Reference) (OtherComp :type Primitive%20Component%20Object%20Reference) (OtherBodyIndex :type Integer) (bFromSweep :type Boolean) (SweepResult :type Hit%20Result%20Structure%20%28by%20ref%29))
  ;[0 0.4219 0.05633] X+90
  (bind _asbp_player_pawn_1 (Utilities|Casting|CastToBP_PlayerPawn_1 OtherActor))
  (Variables|Default|SetAs%20BP%20Player%20Pawn _asbp_player_pawn_1)
  (Variables|Default|SetCurrentRotator "0.000000, 0,90.000000")
  (Variables|Default|SetcanRotate true))

(event OnComponentBeginOverlap(X+90/2)
  (params (OverlappedComponent :type Primitive%20Component%20Object%20Reference) (OtherActor :type Actor%20Object%20Reference) (OtherComp :type Primitive%20Component%20Object%20Reference) (OtherBodyIndex :type Integer) (bFromSweep :type Boolean) (SweepResult :type Hit%20Result%20Structure%20%28by%20ref%29))
  ;[0 0.4219 0.05633] X+90
  (bind _asbp_player_pawn_1 (Utilities|Casting|CastToBP_PlayerPawn_1 OtherActor))
  (Variables|Default|SetAs%20BP%20Player%20Pawn _asbp_player_pawn_1)
  (Variables|Default|SetCurrentRotator "0.000000, 0,90.000000")
  (Variables|Default|SetcanRotate true))

(event OnComponentBeginOverlap(X+90/3)
  (params (OverlappedComponent :type Primitive%20Component%20Object%20Reference) (OtherActor :type Actor%20Object%20Reference) (OtherComp :type Primitive%20Component%20Object%20Reference) (OtherBodyIndex :type Integer) (bFromSweep :type Boolean) (SweepResult :type Hit%20Result%20Structure%20%28by%20ref%29))
  ;[0 0.4219 0.05633] X+90
  (bind _asbp_player_pawn_1 (Utilities|Casting|CastToBP_PlayerPawn_1 OtherActor))
  (Variables|Default|SetAs%20BP%20Player%20Pawn _asbp_player_pawn_1)
  (Variables|Default|SetCurrentRotator "0.000000, 0,90.000000")
  (Variables|Default|SetcanRotate true))

(event OnComponentBeginOverlap(X+90/4)
  (params (OverlappedComponent :type Primitive%20Component%20Object%20Reference) (OtherActor :type Actor%20Object%20Reference) (OtherComp :type Primitive%20Component%20Object%20Reference) (OtherBodyIndex :type Integer) (bFromSweep :type Boolean) (SweepResult :type Hit%20Result%20Structure%20%28by%20ref%29))
  ;[0 0.4219 0.05633] X+90
  (bind _asbp_player_pawn_1 (Utilities|Casting|CastToBP_PlayerPawn_1 OtherActor))
  (Variables|Default|SetAs%20BP%20Player%20Pawn _asbp_player_pawn_1)
  (Variables|Default|SetCurrentRotator "0.000000, 0,90.000000")
  (Variables|Default|SetcanRotate true))

(event OnComponentBeginOverlap(X-90/3)
  (params (OverlappedComponent :type Primitive%20Component%20Object%20Reference) (OtherActor :type Actor%20Object%20Reference) (OtherComp :type Primitive%20Component%20Object%20Reference) (OtherBodyIndex :type Integer) (bFromSweep :type Boolean) (SweepResult :type Hit%20Result%20Structure%20%28by%20ref%29))
  ;[0.4219 0 0.01549] X-90
  (bind _asbp_player_pawn_1 (Utilities|Casting|CastToBP_PlayerPawn_1 OtherActor))
  (Variables|Default|SetAs%20BP%20Player%20Pawn _asbp_player_pawn_1)
  (Variables|Default|SetCurrentRotator "0.000000, 0,-90.000000")
  (Variables|Default|SetcanRotate true))

(event OnComponentBeginOverlap(X-90/4)
  (params (OverlappedComponent :type Primitive%20Component%20Object%20Reference) (OtherActor :type Actor%20Object%20Reference) (OtherComp :type Primitive%20Component%20Object%20Reference) (OtherBodyIndex :type Integer) (bFromSweep :type Boolean) (SweepResult :type Hit%20Result%20Structure%20%28by%20ref%29))
  ;[0.4219 0 0.01549] X-90
  (bind _asbp_player_pawn_1 (Utilities|Casting|CastToBP_PlayerPawn_1 OtherActor))
  (Variables|Default|SetAs%20BP%20Player%20Pawn _asbp_player_pawn_1)
  (Variables|Default|SetCurrentRotator "0.000000, 0,-90.000000")
  (Variables|Default|SetcanRotate true))

(event OnComponentBeginOverlap(X-90/2)
  (params (OverlappedComponent :type Primitive%20Component%20Object%20Reference) (OtherActor :type Actor%20Object%20Reference) (OtherComp :type Primitive%20Component%20Object%20Reference) (OtherBodyIndex :type Integer) (bFromSweep :type Boolean) (SweepResult :type Hit%20Result%20Structure%20%28by%20ref%29))
  ;[0.4219 0 0.01549] X-90
  (bind _asbp_player_pawn_1 (Utilities|Casting|CastToBP_PlayerPawn_1 OtherActor))
  (Variables|Default|SetAs%20BP%20Player%20Pawn _asbp_player_pawn_1)
  (Variables|Default|SetCurrentRotator "0.000000, 0,-90.000000")
  (Variables|Default|SetcanRotate true))

(event OnComponentBeginOverlap(X-90/1)
  (params (OverlappedComponent :type Primitive%20Component%20Object%20Reference) (OtherActor :type Actor%20Object%20Reference) (OtherComp :type Primitive%20Component%20Object%20Reference) (OtherBodyIndex :type Integer) (bFromSweep :type Boolean) (SweepResult :type Hit%20Result%20Structure%20%28by%20ref%29))
  ;[0.4219 0 0.01549] X-90
  (bind _asbp_player_pawn_1 (Utilities|Casting|CastToBP_PlayerPawn_1 OtherActor))
  (Variables|Default|SetAs%20BP%20Player%20Pawn _asbp_player_pawn_1)
  (Variables|Default|SetCurrentRotator "0.000000, 0,-90.000000")
  (Variables|Default|SetcanRotate true))

(event OnComponentBeginOverlap(Y+90/X/Z/2)
  (params (OverlappedComponent :type Primitive%20Component%20Object%20Reference) (OtherActor :type Actor%20Object%20Reference) (OtherComp :type Primitive%20Component%20Object%20Reference) (OtherBodyIndex :type Integer) (bFromSweep :type Boolean) (SweepResult :type Hit%20Result%20Structure%20%28by%20ref%29))
  (bind _asbp_player_pawn_1 (Utilities|Casting|CastToBP_PlayerPawn_1 OtherActor))
  (Variables|Default|SetAs%20BP%20Player%20Pawn _asbp_player_pawn_1)
  (Variables|Default|SetCurrentRotator "-90.000000,0.000000,0.000000")
  (Variables|Default|SetcanRotate true))

(event OnComponentBeginOverlap(Y+90/X/Z/4)
  (params (OverlappedComponent :type Primitive%20Component%20Object%20Reference) (OtherActor :type Actor%20Object%20Reference) (OtherComp :type Primitive%20Component%20Object%20Reference) (OtherBodyIndex :type Integer) (bFromSweep :type Boolean) (SweepResult :type Hit%20Result%20Structure%20%28by%20ref%29))
  (bind _asbp_player_pawn_1 (Utilities|Casting|CastToBP_PlayerPawn_1 OtherActor))
  (Variables|Default|SetAs%20BP%20Player%20Pawn _asbp_player_pawn_1)
  (Variables|Default|SetCurrentRotator "-90.000000,90.000000,90.000000")
  (Variables|Default|SetcanRotate true))

(event OnComponentBeginOverlap(Y+90/X/Z/1)
  (params (OverlappedComponent :type Primitive%20Component%20Object%20Reference) (OtherActor :type Actor%20Object%20Reference) (OtherComp :type Primitive%20Component%20Object%20Reference) (OtherBodyIndex :type Integer) (bFromSweep :type Boolean) (SweepResult :type Hit%20Result%20Structure%20%28by%20ref%29))
  (bind _asbp_player_pawn_1 (Utilities|Casting|CastToBP_PlayerPawn_1 OtherActor))
  (Variables|Default|SetAs%20BP%20Player%20Pawn _asbp_player_pawn_1)
  (Variables|Default|SetCurrentRotator "-90.000000,-90.000000,90.000000")
  (Variables|Default|SetcanRotate true))

(event OnComponentBeginOverlap(Y+90/X/Z/3)
  (params (OverlappedComponent :type Primitive%20Component%20Object%20Reference) (OtherActor :type Actor%20Object%20Reference) (OtherComp :type Primitive%20Component%20Object%20Reference) (OtherBodyIndex :type Integer) (bFromSweep :type Boolean) (SweepResult :type Hit%20Result%20Structure%20%28by%20ref%29))
  (bind _asbp_player_pawn_1 (Utilities|Casting|CastToBP_PlayerPawn_1 OtherActor))
  (Variables|Default|SetAs%20BP%20Player%20Pawn _asbp_player_pawn_1)
  (Variables|Default|SetCurrentRotator "90.000000, 0, 0")
  (Variables|Default|SetcanRotate true))

(event OnComponentBeginOverlap(Y-90/X/Z/1)
  (params (OverlappedComponent :type Primitive%20Component%20Object%20Reference) (OtherActor :type Actor%20Object%20Reference) (OtherComp :type Primitive%20Component%20Object%20Reference) (OtherBodyIndex :type Integer) (bFromSweep :type Boolean) (SweepResult :type Hit%20Result%20Structure%20%28by%20ref%29))
  ;[1 1 1] Comment
  (bind _asbp_player_pawn_1 (Utilities|Casting|CastToBP_PlayerPawn_1 OtherActor))
  (Variables|Default|SetAs%20BP%20Player%20Pawn _asbp_player_pawn_1)
  (Variables|Default|SetCurrentRotator "-90.000000,0.000000,0.000000")
  (Variables|Default|SetcanRotate true))

(event OnComponentBeginOverlap(Y-90/X/Z/2)
  (params (OverlappedComponent :type Primitive%20Component%20Object%20Reference) (OtherActor :type Actor%20Object%20Reference) (OtherComp :type Primitive%20Component%20Object%20Reference) (OtherBodyIndex :type Integer) (bFromSweep :type Boolean) (SweepResult :type Hit%20Result%20Structure%20%28by%20ref%29))
  ;[1 1 1] Comment
  (bind _asbp_player_pawn_1 (Utilities|Casting|CastToBP_PlayerPawn_1 OtherActor))
  (Variables|Default|SetAs%20BP%20Player%20Pawn _asbp_player_pawn_1)
  (Variables|Default|SetCurrentRotator "90.000000,0.000000,0.000000")
  (Variables|Default|SetcanRotate true))

(event OnComponentBeginOverlap(Y-90/X/Z/3)
  (params (OverlappedComponent :type Primitive%20Component%20Object%20Reference) (OtherActor :type Actor%20Object%20Reference) (OtherComp :type Primitive%20Component%20Object%20Reference) (OtherBodyIndex :type Integer) (bFromSweep :type Boolean) (SweepResult :type Hit%20Result%20Structure%20%28by%20ref%29))
  (bind _asbp_player_pawn_1 (Utilities|Casting|CastToBP_PlayerPawn_1 OtherActor))
  (Variables|Default|SetAs%20BP%20Player%20Pawn _asbp_player_pawn_1)
  (Variables|Default|SetCurrentRotator "90.000000,-90.000000,-270.000000")
  (Variables|Default|SetcanRotate true))

(event OnComponentBeginOverlap(Y-90/X/Z/4)
  (params (OverlappedComponent :type Primitive%20Component%20Object%20Reference) (OtherActor :type Actor%20Object%20Reference) (OtherComp :type Primitive%20Component%20Object%20Reference) (OtherBodyIndex :type Integer) (bFromSweep :type Boolean) (SweepResult :type Hit%20Result%20Structure%20%28by%20ref%29))
  (bind _asbp_player_pawn_1 (Utilities|Casting|CastToBP_PlayerPawn_1 OtherActor))
  (Variables|Default|SetAs%20BP%20Player%20Pawn _asbp_player_pawn_1)
  (Variables|Default|SetCurrentRotator "-90.000000,180.000000,270.000000")
  (Variables|Default|SetcanRotate true))

(event OnComponentBeginOverlap(Box)
  (params (OverlappedComponent :type Primitive%20Component%20Object%20Reference) (OtherActor :type Actor%20Object%20Reference) (OtherComp :type Primitive%20Component%20Object%20Reference) (OtherBodyIndex :type Integer) (bFromSweep :type Boolean) (SweepResult :type Hit%20Result%20Structure%20%28by%20ref%29))
  (Transformation|AttachActorToActor OtherActor self "None" "KeepWorld" "KeepWorld" "KeepWorld" true))

(event Custom|RotateCube
  (bind _defaultsceneroot (Variables|Default|GetDefaultSceneRoot))
  (bind _currentrotator (Variables|Default|GetCurrentRotator))
  (bind _returnvalue (Transformation|GetWorldRotation _defaultsceneroot))
  (Components|MoveComponentTo _defaultsceneroot "0, 0, 0" (Math|Rotator|MakeRotator (+ (.roll _returnvalue) (.roll _currentrotator)) (+ (.pitch _returnvalue) (.pitch _currentrotator)) (+ (.yaw _returnvalue) (.yaw _currentrotator))) true true 1.0 false)
  (Variables|Default|SetcanRotate false))

(event EventBeginPlay
  (bind _asbp_player_pawn_1 (Utilities|Casting|CastToBP_PlayerPawn_1 (Game|Player|GetPlayerPawn 0)))
  (Variables|Default|SetAs%20BP%20Player%20Pawn _asbp_player_pawn_1))

(fn ConstructionScript)