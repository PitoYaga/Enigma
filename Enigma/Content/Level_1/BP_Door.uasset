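; Level exit door that changes material once the game mode flags the level as passed.
; BeginPlay caches the GM_GameMode, and Tick polls its LevelPassed flag, reapplying the projectile material to the door every frame while true.
; Overlapping the Box while passed only prints "Next Level"; no level load occurs.
; The construction script checks the same flag to apply Green, though that reference is only assigned at BeginPlay.
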(event OnComponentBeginOverlap(Box)
  (params (OverlappedComponent :type Primitive%20Component%20Object%20Reference) (OtherActor :type Actor%20Object%20Reference) (OtherComp :type Primitive%20Component%20Object%20Reference) (OtherBodyIndex :type Integer) (bFromSweep :type Boolean) (SweepResult :type Hit%20Result%20Structure%20%28by%20ref%29))
  (if (Variables|/Game/Efe/GM_GameMode.GM_GameMode_C|GetLevelPassed (Variables|Default|GetAs%20GM%20Game%20Mode))
    (Development|PrintString "Next Level")))

(event EventBeginPlay
  (bind _asgm_game_mode (Utilities|Casting|CastToGM_GameMode (Game|GetGameMode)))
  (Variables|Default|SetAs%20GM%20Game%20Mode _asgm_game_mode))

(event EventTick
  (params (DeltaSeconds :type Float%20%28single-precision%29))
  (if (Variables|/Game/Efe/GM_GameMode.GM_GameMode_C|GetLevelPassed (Variables|Default|GetAs%20GM%20Game%20Mode))
    (Rendering|Material|SetMaterial (Variables|Default|GetDoor) 0 "/Game/UnrealContent/FPWeapon/Materials/FirstPersonProjectileMaterial.FirstPersonProjectileMaterial")))

(fn ConstructionScript
  (if (Variables|/Game/Efe/GM_GameMode.GM_GameMode_C|GetLevelPassed (Variables|Default|GetAs%20GM%20Game%20Mode))
    (Rendering|Material|SetMaterial (Variables|Default|GetDoor) 0 "/Game/Level_1/Materials/Green.Green")))