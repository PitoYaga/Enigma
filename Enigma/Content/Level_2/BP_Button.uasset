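; Puzzle button for Level 2 with a configurable mesh, forming part of up to three successive combinations tracked by GM_GameMode_2.
; Every Tick it polls and clears BP_PlayerPawn_2 flags and sets its "Clickable" tag when it belongs to the current combination.
; Correct presses turn it blue and raise the shared count, advancing the combination at three with a green flash.
; Wrong presses flash red and reset progress; the timeout is disconnected.
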(event Custom|WrongButton
  (bind _buttonshape (Variables|Default|GetButtonShape))
  (bind _as_gm_game_mode_2 (Variables|Default|GetAs%20GM%20Game%20Mode%202))
  (bind _as_bp_player_pawn_2 (Variables|Default|GetAs%20BP%20Player%20Pawn%202))
  ;[0.276 0.003848 0] Wrong Button
  (if (Variables|/Game/Level_2/BP_PlayerPawn_2.BP_PlayerPawn_2_C|GetWrongButton _as_bp_player_pawn_2)
    (Variables|/Game/Level_2/BP_PlayerPawn_2.BP_PlayerPawn_2_C|SetWrongButton _as_bp_player_pawn_2 false)
    (Rendering|Material|SetMaterial _buttonshape 0 "/Game/Level_1/Materials/RedEmmision.RedEmmision")
    (Utilities|FlowControl|Delay 0.5)
    (Rendering|Material|SetMaterial _buttonshape 0 "/Game/UnrealContent/FPWeapon/Materials/BaseMaterial.BaseMaterial")
    (Utilities|FlowControl|Sequence
      (:then_1
        (Utilities|FlowControl|Sequence
          (:then_0
            (Variables|/Game/Level_2/GM_GameMode_2.GM_GameMode_2_C|SetCorrectButton _as_gm_game_mode_2 0))
          (:then_1
            (Variables|/Game/Level_2/GM_GameMode_2.GM_GameMode_2_C|SetCurrentCombination _as_gm_game_mode_2 1))
          (:then_2
            (Variables|Default|SetPuzzleStarted false))))
      (:then_2
        ;[0.5156 0 0.4133] Show Combination
        (Rendering|Material|SetMaterial (Variables|Default|GetButtonShape) 0 "/Game/UnrealContent/FPWeapon/Materials/FirstPersonProjectileMaterial.FirstPersonProjectileMaterial")
        (Utilities|FlowControl|Delay 1.0)
        (Rendering|Material|SetMaterial (Variables|Default|GetButtonShape) 0 "/Game/UnrealContent/FPWeapon/Materials/BaseMaterial.BaseMaterial")))))

(event Custom|TimeOut
  ;[0.3958 0.3333 0] TimeOut
)

(event Custom|CorrectButton
  (bind _as_gm_game_mode_2 (Variables|Default|GetAs%20GM%20Game%20Mode%202))
  (bind _as_bp_player_pawn_2 (Variables|Default|GetAs%20BP%20Player%20Pawn%202))
  ;[0.1689 0.401 0.1699] Correct Button
  (if (Variables|/Game/Level_2/BP_PlayerPawn_2.BP_PlayerPawn_2_C|GetCorrectButton _as_bp_player_pawn_2)
    (Variables|/Game/Level_2/BP_PlayerPawn_2.BP_PlayerPawn_2_C|SetCorrectButton _as_bp_player_pawn_2 false)
    (Utilities|FlowControl|Sequence
      (:then_0
        (Rendering|Material|SetMaterial (Variables|Default|GetButtonShape) 0 "/Game/Level_1/Materials/BlueEmmision.BlueEmmision")
        (Variables|/Game/Level_2/GM_GameMode_2.GM_GameMode_2_C|SetCorrectButton _as_gm_game_mode_2 (+ (Variables|/Game/Level_2/GM_GameMode_2.GM_GameMode_2_C|GetCorrectButton _as_gm_game_mode_2) 1))
        (Development|PrintString (Utilities|GetDisplayName self)))
      (:then_1
        (Variables|Default|SetPuzzleStarted true)))))

(event Custom|CalculateCombination
  (bind _as_gm_game_mode_2 (Variables|Default|GetAs%20GM%20Game%20Mode%202))
  ;[0 0.3906 0.3664] Combination Calculator
  (if (== (Variables|/Game/Level_2/GM_GameMode_2.GM_GameMode_2_C|GetCorrectButton _as_gm_game_mode_2) 3)
    (Variables|/Game/Level_2/GM_GameMode_2.GM_GameMode_2_C|SetCorrectButton _as_gm_game_mode_2 0)
    (Variables|/Game/Level_2/GM_GameMode_2.GM_GameMode_2_C|SetCurrentCombination _as_gm_game_mode_2 (+ (Variables|/Game/Level_2/GM_GameMode_2.GM_GameMode_2_C|GetCurrentCombination _as_gm_game_mode_2) 1))
    (Rendering|Material|SetMaterial (Variables|Default|GetButtonShape) 0 "/Game/Level_1/Materials/GreenEmmision.GreenEmmision")
    (Utilities|FlowControl|Delay 1.0)
    (Rendering|Material|SetMaterial (Variables|Default|GetButtonShape) 0 "/Game/UnrealContent/FPWeapon/Materials/BaseMaterial.BaseMaterial")))

(event Custom|ShowCombination
  (bind _as_bp_player_pawn_2 (Variables|Default|GetAs%20BP%20Player%20Pawn%202))
  ;[0.5156 0 0.4133] Show Combination
  (if (and (Variables|/Game/Level_2/BP_PlayerPawn_2.BP_PlayerPawn_2_C|GetShowCombination _as_bp_player_pawn_2) true)
    (Variables|/Game/Level_2/BP_PlayerPawn_2.BP_PlayerPawn_2_C|SetShowCombination _as_bp_player_pawn_2 false)
    (Rendering|Material|SetMaterial (Variables|Default|GetButtonShape) 0 "/Game/UnrealContent/FPWeapon/Materials/FirstPersonProjectileMaterial.FirstPersonProjectileMaterial")
    (Utilities|FlowControl|Delay 1.0)
    (Rendering|Material|SetMaterial (Variables|Default|GetButtonShape) 0 "/Game/UnrealContent/FPWeapon/Materials/BaseMaterial.BaseMaterial")))

(event Custom|Combinations
  (bind _as_gm_game_mode_2 (Variables|Default|GetAs%20GM%20Game%20Mode%202))
  (bind _currentcombination (Variables|/Game/Level_2/GM_GameMode_2.GM_GameMode_2_C|GetCurrentCombination _as_gm_game_mode_2))
  ;[0 0.1772 0.4948] Combinations
  (if (Math|Boolean|ORBoolean (and (Variables|Default|GetCombination_1) (== _currentcombination 1)) (and (Variables|Default|GetCombination_2) (== _currentcombination 2)) (and (Variables|Default|GetCombination_3) (== _currentcombination 3)))
    (bind _output_get (Variables|Default|SetActorTag "Clickable"))
    (else
      (bind _output_get_2 (Variables|Default|SetActorTag "None"))))
  (Variables|Default|SetTags (Utilities|Array|MakeArray _output_get _output_get_2)))

(event EventBeginPlay
  (bind _asbp_player_pawn_2 (Utilities|Casting|CastToBP_PlayerPawn_2 (Game|Player|GetPlayerPawn 0)))
  (Variables|Default|SetAs%20BP%20Player%20Pawn%202 _asbp_player_pawn_2)
  (bind _asgm_game_mode_2 (Utilities|Casting|CastToGM_GameMode_2 (Game|GetGameMode)))
  (Variables|Default|SetAs%20GM%20Game%20Mode%202 _asgm_game_mode_2))

(event EventTick
  (params (DeltaSeconds :type Float%20%28single-precision%29))
  (Utilities|FlowControl|Sequence
    (:then_0
      (CallFunction|CorrectButton)
      (CallFunction|ShowCombination)
      (Development|PrintString "interface kullan"))
    (:then_1
      (CallFunction|WrongButton)
      (CallFunction|TimeOut))
    (:then_2
      (CallFunction|Combinations)
      (CallFunction|CalculateCombination))))

(fn ConstructionScript
  (Rendering|Material|SetMaterial (Variables|Default|GetButtonShape) 0 "/Game/UnrealContent/FPWeapon/Materials/BaseMaterial.BaseMaterial")
  (Components|StaticMesh|SetStaticMesh (Variables|Default|GetButtonShape) (Variables|Default|GetShape)))