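; Level 3 puzzle button for a multi-stage combination puzzle, with progress held in GM_GameMode_2.
; Each Tick, combination flags and current stage set its Clickable tag, and pawn-requested hints flash clickable buttons yellow.
; Interact reads game-mode true/false flags to count a blue hit or flash red and reset progress.
; Three hits make every button flash green and increment the shared stage counter, hence stage values 1, 7, 13.
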(event Custom|WrongButton
  (bind _as_gm_game_mode_2 (Variables|Default|GetAs%20GM%20Game%20Mode%202))
  (bind _buttonshape (Variables|Default|GetButtonShape))
  ;[0.276 0.003848 0] Wrong Button
  (if (Variables|/Game/Level_3/GM_GameMode_2.GM_GameMode_2_C|GetFalseButton (Variables|Default|GetAs%20GM%20Game%20Mode%202))
    (Rendering|Material|SetMaterial _buttonshape 0 "/Game/Level_1/Materials/RedEmmision.RedEmmision")
    (Utilities|FlowControl|Delay 1.0)
    (Rendering|Material|SetMaterial _buttonshape 0 "/Game/Level_3/ButtonBase.ButtonBase")
    (Utilities|FlowControl|Sequence
      (:then_0
        (Variables|/Game/Level_3/GM_GameMode_2.GM_GameMode_2_C|SetCorrectButton _as_gm_game_mode_2 0)
        (Variables|/Game/Level_3/GM_GameMode_2.GM_GameMode_2_C|SetCurrentCombination _as_gm_game_mode_2 1)
        (Variables|Default|SetPuzzleStarted false)
        (CallFunction|Combinations))
      (:then_1
        (Variables|Default|SetSound "/Game/Level_3/Sounds/wrong_button.wrong_button")))))

(event Custom|TimeOut
  ;[0.3958 0.3333 0] TimeOut
  (if (Variables|Default|GetPuzzleStarted)
    (Variables|Default|SetPuzzleStarted false)
    (Utilities|FlowControl|Delay 5.0)))

(event Custom|CorrectButton
  (bind _as_gm_game_mode_2 (Variables|Default|GetAs%20GM%20Game%20Mode%202))
  ;[0.1689 0.401 0.1699] Correct Button
  (if (Variables|/Game/Level_3/GM_GameMode_2.GM_GameMode_2_C|GetTrueButton (Variables|Default|GetAs%20GM%20Game%20Mode%202))
    (Utilities|FlowControl|DoOnce false
      (:Completed
        (Variables|Default|SetPuzzleStarted true)
        (Rendering|Material|SetMaterial (Variables|Default|GetButtonShape) 0 "/Game/Level_1/Materials/BlueEmmision.BlueEmmision")
        (Utilities|FlowControl|Sequence
          (:then_0
            (Variables|/Game/Level_3/GM_GameMode_2.GM_GameMode_2_C|SetCorrectButton _as_gm_game_mode_2 (+ (Variables|/Game/Level_3/GM_GameMode_2.GM_GameMode_2_C|GetCorrectButton _as_gm_game_mode_2) 1))
            (CallFunction|Combinations))
          (:then_1
            (if (<= (Variables|/Game/Level_3/GM_GameMode_2.GM_GameMode_2_C|GetCorrectButton _as_gm_game_mode_2) 2)
              (Variables|Default|SetSound "/Game/Level_3/Sounds/ButtonClick.ButtonClick"))))))))

(event Custom|CalculateCombination
  ;[0 0.3906 0.3664] Combination Calculator
  (if (== (Variables|/Game/Level_3/GM_GameMode_2.GM_GameMode_2_C|GetCorrectButton (Variables|Default|GetAs%20GM%20Game%20Mode%202)) 3)
    (bind _outactors (Actor|GetAllActorsOfClass "BP_Button_C"))
    (CallFunction|CombinationFinish _outactors)))

(event Custom|ShowCombination
  (bind _as_bp_player_pawn_2 (Variables|Default|GetAs%20BP%20Player%20Pawn%202))
  ;[0.5156 0 0.4133] Show Combination
  (if (Math|Boolean|ANDBoolean (Variables|/Game/Level_3/BP_PlayerPawn_2.BP_PlayerPawn_2_C|GetShowCombination _as_bp_player_pawn_2) (Actor|ActorHasTag "Clickable") (> (Variables|Default|GetHintCount) 0))
    (Rendering|Material|SetMaterial (Variables|Default|GetButtonShape) 0 "/Game/Level_1/Materials/YellowEmmision.YellowEmmision")
    (Utilities|FlowControl|Delay 0.5)
    (Rendering|Material|SetMaterial (Variables|Default|GetButtonShape) 0 "/Game/Level_3/ButtonBase.ButtonBase")
    (Variables|/Game/Level_3/BP_PlayerPawn_2.BP_PlayerPawn_2_C|SetShowCombination _as_bp_player_pawn_2 false)
    (Variables|/Game/Level_3/GM_GameMode_2.GM_GameMode_2_C|SetCorrectButton (Variables|Default|GetAs%20GM%20Game%20Mode%202) 0)
    (Math|Integer|DecrementInt (Variables|Default|GetHintCount))))

(event Custom|Combinations
  (bind _as_gm_game_mode_2 (Variables|Default|GetAs%20GM%20Game%20Mode%202))
  (bind _currentcombination (Variables|/Game/Level_3/GM_GameMode_2.GM_GameMode_2_C|GetCurrentCombination _as_gm_game_mode_2))
  ;[0 0.1772 0.4948] Combinations
  (CallFunction|CalculateCombination)
  (if (Math|Boolean|ORBoolean (and (Variables|Default|GetCombination_1) (== _currentcombination 1)) (and (Variables|Default|GetCombination_2) (== _currentcombination 7)) (and (Variables|Default|GetCombination_3) (== _currentcombination 13)))
    (bind _output_get (Variables|Default|SetActorTag "Clickable"))
    (else
      (bind _output_get_2 (Variables|Default|SetActorTag "NotClick"))))
  (Variables|Default|SetTags (Utilities|Array|MakeArray _output_get _output_get_2)))

(event Custom|CombinationFinish
  (bind _as_gm_game_mode_2 (Variables|Default|GetAs%20GM%20Game%20Mode%202))
  (bind _as_gm_game_mode_2_2 (Variables|Default|GetAs%20GM%20Game%20Mode%202))
  ;[1 1 1] CombinationComplated
  (Variables|/Game/Level_3/GM_GameMode_2.GM_GameMode_2_C|SetCorrectButton _as_gm_game_mode_2_2 0)
  (Rendering|Material|SetMaterial (Variables|Default|GetButtonShape) 0 "/Game/Level_1/Materials/GreenEmmision.GreenEmmision")
  (Audio|PlaySoundatLocation "/Game/Level_3/Sounds/CorrectButton.CorrectButton" (Transformation|GetActorLocation) "0, 0, 0" 1.0 1.0 0.0 0 0 0 0)
  (Utilities|FlowControl|Delay 1.0)
  (Rendering|Material|SetMaterial (Variables|Default|GetButtonShape) 0 "/Game/Level_3/ButtonBase.ButtonBase")
  (Math|Integer|IncrementInt (Variables|/Game/Level_3/GM_GameMode_2.GM_GameMode_2_C|GetCurrentCombination _as_gm_game_mode_2_2)
    (:%20%20
      ;[0.1689 0.401 0.1699] Correct Button
      (Utilities|FlowControl|DoOnce false) ; enters at Reset
    )))

(event EventInteract
  (CallFunction|CorrectButton)
  (CallFunction|WrongButton)
  (Audio|PlaySoundatLocation (Variables|Default|GetSound) (Transformation|GetActorLocation) "0, 0, 0" 1.0 1.0 0.0 0 0 0 0))

(event EventBeginPlay
  (bind _asbp_player_pawn_2 (Utilities|Casting|CastToBP_PlayerPawn_2 (Game|Player|GetPlayerPawn 0)))
  (Variables|Default|SetAs%20BP%20Player%20Pawn%202 _asbp_player_pawn_2)
  (bind _asgm_game_mode_2 (Utilities|Casting|CastToGM_GameMode_2 (Game|GetGameMode)))
  (Variables|Default|SetAs%20GM%20Game%20Mode%202 _asgm_game_mode_2)
  (CallFunction|Combinations)
  (Rendering|Material|SetMaterial (Variables|Default|GetButtonShape) 0 "/Game/Level_3/ButtonBase.ButtonBase"))

(event EventTick
  (params (DeltaSeconds :type Float%20%28single-precision%29))
  (CallFunction|Combinations)
  (CallFunction|ShowCombination))

(fn ConstructionScript
  (Rendering|Material|SetMaterial (Variables|Default|GetButtonShape) 0 "/Game/Level_3/ButtonBase.ButtonBase")
  (Components|StaticMesh|SetStaticMesh (Variables|Default|GetButtonShape) (Variables|Default|GetShape)))